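; BP_Master_Terminal is a terminal Blueprint whose screen and state reflect the lock state of the objects it references.
; On BeginPlay it caches the first BP_TerminalController found in the level.
; CheckIfDoorStillLocked loops over LockedObjects, switching the terminal widget's page and setting UnlockedOrDisabled from each Locked flag.
; Each iteration overwrites the previous one, so only the last object determines the final state.
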(event `self.ReceiveBeginPlay`
  ;[1 1 1] Set a reference to terminal controller
  (bind _outactors (`GameplayStatics.GetAllActorsOfClass` "/Game/WISTerminals/Blueprints/BP_TerminalController.BP_TerminalController_C"))
  (set `self.TerminalController` (`|GetArrayItem` _outactors)))

(fn `CheckIfDoorStillLocked`
  (bind _terminalswitch (`/Game/WISTerminals/UserInterface/UI_Keypad_Terminal.TerminalSwitch` (`self.TerminalInterfaceInstance`)))
  (for _array_element (`self.LockedObjects`)
    (if (`/Game/WISTerminals/Blueprints/Core/BP_Master_LinkedObject.Locked` _array_element)
      (`WidgetSwitcher.SetActiveWidgetIndex` _terminalswitch 0)
      (set `self.UnlockedOrDisabled` false)
      (else
        (`WidgetSwitcher.SetActiveWidgetIndex` _terminalswitch 2)
        (set `self.UnlockedOrDisabled` true)))))

(fn `UserConstructionScript`)